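; BP_KnifeTrap is a one-shot trap that launches four knives when an actor first overlaps it.
; On that overlap, ActivateTrap enables physics on the knife components and applies an equal impulse along the Direction component's forward vector.
; Any knife's hit event opens the DeathMenu level, whatever it struck.
; Neither overlap nor hit filters for the player, as the dragon-player cast and Player tag checks are unconnected.
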(event `self.ReceiveActorBeginOverlap`
  (params (OtherActor :type "Actor Object Reference"))
  (if (not (`self.bIsTriggered`))
    (`self.ActivateTrap`)
    (set `self.bIsTriggered` true)))

(event `ActivateTrap`
  (bind _knife2 (`self.Knife2`))
  (bind _knife3 (`self.Knife3`))
  (bind _knife4 (`self.Knife4`))
  (bind _knife1 (`self.Knife1`))
  (bind _returnvalue (* (`SceneComponent.GetForwardVector` (`self.Direction`)) 2500.0))
  (`PrimitiveComponent.SetSimulatePhysics` _knife1 true)
  (`PrimitiveComponent.SetSimulatePhysics` _knife2 true)
  (`PrimitiveComponent.SetSimulatePhysics` _knife3 true)
  (`PrimitiveComponent.SetSimulatePhysics` _knife4 true)
  (`PrimitiveComponent.AddImpulse` _knife1 _returnvalue "None" false)
  (`PrimitiveComponent.AddImpulse` _knife2 _returnvalue "None" false)
  (`PrimitiveComponent.AddImpulse` _knife3 _returnvalue "None" false)
  (`PrimitiveComponent.AddImpulse` _knife4 _returnvalue "None" false))

(event `self.Knife4.OnComponentHit`
  (params (HitComponent :type "PrimitiveComponent Object Reference") (OtherActor :type "Actor Object Reference") (OtherComp :type "PrimitiveComponent Object Reference") (NormalImpulse :type "Vector Structure") (Hit :type "HitResult Structure (by ref)"))
  (`GameplayStatics.OpenLevel` "DeathMenu" :!label _label))

(event `self.Knife3.OnComponentHit`
  (params (HitComponent :type "PrimitiveComponent Object Reference") (OtherActor :type "Actor Object Reference") (OtherComp :type "PrimitiveComponent Object Reference") (NormalImpulse :type "Vector Structure") (Hit :type "HitResult Structure (by ref)"))
  (goto _label))

(event `self.Knife2.OnComponentHit`
  (params (HitComponent :type "PrimitiveComponent Object Reference") (OtherActor :type "Actor Object Reference") (OtherComp :type "PrimitiveComponent Object Reference") (NormalImpulse :type "Vector Structure") (Hit :type "HitResult Structure (by ref)"))
  (goto _label))

(event `self.Knife1.OnComponentHit`
  (params (HitComponent :type "PrimitiveComponent Object Reference") (OtherActor :type "Actor Object Reference") (OtherComp :type "PrimitiveComponent Object Reference") (NormalImpulse :type "Vector Structure") (Hit :type "HitResult Structure (by ref)"))
  (goto _label))

(fn `UserConstructionScript`)