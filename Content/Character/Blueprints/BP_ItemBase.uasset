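; BP_ItemBase is an item actor that bobs up and down in the world, apparently meant as a base for pickups.
; Tick calls HoverMovement, which adds the sine of time since creation to the current Z each frame, unscaled by delta time.
; Unconnected graph fragments sketch a pickup that casts to BP_DragonPlayer, adds a sword weapon and destroys the item, but overlap currently does nothing.
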(event `self.ReceiveActorBeginOverlap`
  (params (OtherActor :type "Actor Object Reference")))

(event `self.ReceiveTick`
  (params (DeltaSeconds :type "Float (single-precision)"))
  (`self.HoverMovement`))

(fn `HoverMovement`
  (bind (_returnvalue_x _returnvalue_y _returnvalue_z) (`KismetMathLibrary.BreakVector` (`self.K2_GetActorLocation`)))
  (`self.K2_SetActorLocation` (`KismetMathLibrary.MakeVector` _returnvalue_x _returnvalue_y (+ _returnvalue_z (* (`KismetMathLibrary.Sin` (`self.GetGameTimeSinceCreation`)) 1.0)))))

(fn `UserConstructionScript`)