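; Wolf spider enemy that chases the DragonCharacter and bites it at close range.
; Tick re-rolls reachable navmesh points around the player and steers straight at them with movement input, without AI pathfinding.
; Within attack range it plays a one-shot animation, then after a delay checks AttackBox overlap to remove a life, restoring the AnimBP and cooling down.
; A hit on the last life starts streaming in the WinMenu level instead.
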(event `self.ReceiveBeginPlay`
  (bind _returnvalue (`GameplayStatics.GetActorOfClass` "/Script/DragonsLair.DragonCharacter")))

(event `self.ReceiveTick`
  (params (DeltaSeconds :type "Float (single-precision)"))
  (bind _returnvalue (- (`NavigationSystemV1.K2_GetRandomReachablePointInRadius` (`SceneComponent.K2_GetComponentLocation` (`Character.Mesh` (stale `self.ReceiveBeginPlay` _returnvalue))) 100.0 null "/Script/NavigationSystem.NavigationQueryFilter") (`self.K2_GetActorLocation`)))
  (bind _returnvalue_2 (`KismetMathLibrary.VSize` _returnvalue))
  (if (and (< _returnvalue_2 3000.0) (> _returnvalue_2 350.0))
    (`self.AddMovementInput` (`KismetMathLibrary.Normal` _returnvalue) (`self.speed`) true)
    (elif (and (< _returnvalue_2 250.0) (`self.canAttack`))
      (set `self.canAttack` false)
      (`SkeletalMeshComponent.PlayAnimation` (`self.Mesh`) "/Game/Character/Modles_Art/Spider/Spider_360/Wolf_Spider_attack_360Wolf_Spider_Armature_Wolf_Spider_Armature_Spider_Attacking.Wolf_Spider_attack_360Wolf_Spider_Armature_Wolf_Spider_Armature_Spider_Attacking" false)
      (`KismetSystemLibrary.Delay` 0.5)
      (if (`PrimitiveComponent.IsOverlappingComponent` (`Character.CapsuleComponent` (stale `self.ReceiveBeginPlay` _returnvalue)) (`self.attackBox`))
        (bind _lives (`DragonCharacter.lives` (stale `self.ReceiveBeginPlay` _returnvalue)))
        (if (<= _lives 1.0)
          (`GameplayStatics.LoadStreamLevel` "WinMenu")
          (else
            (set `DragonCharacter.lives` (- _lives 1.0) (stale `self.ReceiveBeginPlay` _returnvalue))
            (`SkeletalMeshComponent.SetAnimationMode` (`self.Mesh`) "AnimationBlueprint" true :!label _label)
            (`KismetSystemLibrary.Delay` 2.0)
            (set `self.canAttack` true)))
        (else
          (goto _label))))))

(fn `UserConstructionScript`)