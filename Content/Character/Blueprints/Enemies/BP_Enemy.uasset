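; BP_Enemy is an enemy actor that damages the dragon player on contact and ends the level when either side runs out of lives.
; Its AttackTrigger overlap takes one life from a Player-tagged BP_DragonPlayer.
; Tick polls the enemy's own Lives and destroys it at zero.
; Both enemy death and player death lead to opening the MainMenu level; a RestartGame branch is left unconnected.
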(event `self.ReceiveTick`
  (params (DeltaSeconds :type "Float (single-precision)"))
  (if (<= (`self.lives`) 0.0)
    (set `self.isAlive` false)
    (`self.K2_DestroyActor`)
    (`GameplayStatics.OpenLevel` "MainMenu" :!label _label)))

(event `self.attackTrigger.OnComponentBeginOverlap`
  (params (OverlappedComponent :type "PrimitiveComponent Object Reference") (OtherActor :type "Actor Object Reference") (OtherComp :type "PrimitiveComponent Object Reference") (OtherBodyIndex :type Integer) (bFromSweep :type Boolean) (SweepResult :type "HitResult Structure (by ref)"))
  (if (`self.ActorHasTag` OtherActor "Player")
    (bind _asbp_dragon_player (cast `/Game/Character/Blueprints/Player/BP_DragonPlayer` OtherActor))
    (bind _lives (`/Game/Character/Blueprints/Player/BP_DragonPlayer.lives` _asbp_dragon_player))
    (set `/Game/Character/Blueprints/Player/BP_DragonPlayer.lives` (- _lives 1.0) _asbp_dragon_player)
    (if (<= _lives 0.0)
      (goto _label))))

(fn `UserConstructionScript`)