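; Enemy spawner actor that creates backup enemies when the player enters its trigger volumes.
; Each of the two triggers checks for the "Player" tag, then spawns BP_EnemyBackup_Child at its own four spawn points and gives each a default AI controller.
; The triggers have no one-shot guard, so every player re-entry spawns another group.
; A separate KillSelf volume destroys any overlapping actor tagged "Enemy".
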(event `self.EnemySpawnTrigger.OnComponentBeginOverlap`
  (params (OverlappedComponent :type "PrimitiveComponent Object Reference") (OtherActor :type "Actor Object Reference") (OtherComp :type "PrimitiveComponent Object Reference") (OtherBodyIndex :type Integer) (bFromSweep :type Boolean) (SweepResult :type "HitResult Structure (by ref)"))
  (if (`self.ActorHasTag` OtherActor "Player")
    (bind _returnvalue (`|SpawnActorFromClass` "/Game/Character/Blueprints/Enemies/BP_EnemyBackup_Child.BP_EnemyBackup_Child_C" (`SceneComponent.K2_GetComponentToWorld` (`self.EnemySpawnPoint1`)) "AdjustIfPossibleButAlwaysSpawn" "MultiplyWithRoot" null null))
    (`Pawn.SpawnDefaultController` _returnvalue)
    (bind _returnvalue_2 (`|SpawnActorFromClass` "/Game/Character/Blueprints/Enemies/BP_EnemyBackup_Child.BP_EnemyBackup_Child_C" (`SceneComponent.K2_GetComponentToWorld` (`self.EnemySpawnPoint2`)) "AdjustIfPossibleButAlwaysSpawn" "MultiplyWithRoot" null null))
    (`Pawn.SpawnDefaultController` _returnvalue_2)
    (bind _returnvalue_3 (`|SpawnActorFromClass` "/Game/Character/Blueprints/Enemies/BP_EnemyBackup_Child.BP_EnemyBackup_Child_C" (`SceneComponent.K2_GetComponentToWorld` (`self.EnemySpawnPoint3`)) "AdjustIfPossibleButAlwaysSpawn" "MultiplyWithRoot" null null))
    (`Pawn.SpawnDefaultController` _returnvalue_3)
    (bind _returnvalue_4 (`|SpawnActorFromClass` "/Game/Character/Blueprints/Enemies/BP_EnemyBackup_Child.BP_EnemyBackup_Child_C" (`SceneComponent.K2_GetComponentToWorld` (`self.EnemySpawnPoint4`)) "AdjustIfPossibleButAlwaysSpawn" "MultiplyWithRoot" null null))
    (`Pawn.SpawnDefaultController` _returnvalue_4)))

(event `self.EnemySpawnTrigger1.OnComponentBeginOverlap`
  (params (OverlappedComponent :type "PrimitiveComponent Object Reference") (OtherActor :type "Actor Object Reference") (OtherComp :type "PrimitiveComponent Object Reference") (OtherBodyIndex :type Integer) (bFromSweep :type Boolean) (SweepResult :type "HitResult Structure (by ref)"))
  (if (`self.ActorHasTag` OtherActor "Player")
    (bind _returnvalue (`|SpawnActorFromClass` "/Game/Character/Blueprints/Enemies/BP_EnemyBackup_Child.BP_EnemyBackup_Child_C" (`SceneComponent.K2_GetComponentToWorld` (`self.EnemySpawnPoint5`)) "AdjustIfPossibleButAlwaysSpawn" "MultiplyWithRoot" null null))
    (`Pawn.SpawnDefaultController` _returnvalue)
    (bind _returnvalue_2 (`|SpawnActorFromClass` "/Game/Character/Blueprints/Enemies/BP_EnemyBackup_Child.BP_EnemyBackup_Child_C" (`SceneComponent.K2_GetComponentToWorld` (`self.EnemySpawnPoint6`)) "AdjustIfPossibleButAlwaysSpawn" "MultiplyWithRoot" null null))
    (`Pawn.SpawnDefaultController` _returnvalue_2)
    (bind _returnvalue_3 (`|SpawnActorFromClass` "/Game/Character/Blueprints/Enemies/BP_EnemyBackup_Child.BP_EnemyBackup_Child_C" (`SceneComponent.K2_GetComponentToWorld` (`self.EnemySpawnPoint7`)) "AdjustIfPossibleButAlwaysSpawn" "MultiplyWithRoot" null null))
    (`Pawn.SpawnDefaultController` _returnvalue_3)
    (bind _returnvalue_4 (`|SpawnActorFromClass` "/Game/Character/Blueprints/Enemies/BP_EnemyBackup_Child.BP_EnemyBackup_Child_C" (`SceneComponent.K2_GetComponentToWorld` (`self.EnemySpawnPoint8`)) "AdjustIfPossibleButAlwaysSpawn" "MultiplyWithRoot" null null))
    (`Pawn.SpawnDefaultController` _returnvalue_4)))

(event `self.killSelf.OnComponentBeginOverlap`
  (params (OverlappedComponent :type "PrimitiveComponent Object Reference") (OtherActor :type "Actor Object Reference") (OtherComp :type "PrimitiveComponent Object Reference") (OtherBodyIndex :type Integer) (bFromSweep :type Boolean) (SweepResult :type "HitResult Structure (by ref)"))
  (if (`self.ActorHasTag` OtherActor "Enemy")
    (`self.K2_DestroyActor` OtherActor)))

(fn `UserConstructionScript`)