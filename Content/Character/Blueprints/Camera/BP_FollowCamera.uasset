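; Follow camera actor that becomes the first player's view target on BeginPlay and tracks the character along a spline.
; Each tick it projects a point from the player along the camera's forward vector by DistanceToPlayer, then snaps the camera to the closest spline location.
; Yaw follows the spline while pitch and roll stay unchanged, and forward and right vectors are stored.
; Older offset, rail-rig and look-at approaches remain disconnected.
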(event `self.ReceiveBeginPlay`
  (`PlayerController.SetViewTargetWithBlend` (`GameplayStatics.GetPlayerController` 0) self 0.0 "VTBlend_Linear" 0.0 false))

(event `self.ReceiveTick`
  (params (DeltaSeconds :type "Float (single-precision)"))
  (bind _spline (`self.Spline`))
  (bind _camera (`self.Camera`))
  (bind _returnvalue (`SceneComponent.K2_GetComponentRotation` (`self.Camera`)))
  (bind (_returnvalue_roll _returnvalue_pitch) (`KismetMathLibrary.BreakRotator` (`SceneComponent.K2_GetComponentRotation` _camera)))
  (bind _returnvalue_2 (+ (* (`KismetMathLibrary.GetForwardVector` (`SceneComponent.K2_GetComponentRotation` (`self.Camera`))) (`self.distanceToPlayer`)) (`self.K2_GetActorLocation` (`GameplayStatics.GetPlayerCharacter` 0))))
  (bind (_returnvalue_roll_2 _returnvalue_pitch_2 _returnvalue_yaw) (`KismetMathLibrary.BreakRotator` (`SplineComponent.FindRotationClosestToWorldLocation` _spline _returnvalue_2 "World")))
  ; Camera move on spline
  (`SceneComponent.K2_SetWorldRotation` _camera (`KismetMathLibrary.MakeRotator` _returnvalue_roll _returnvalue_pitch _returnvalue_yaw) false false)
  (`SceneComponent.K2_SetWorldLocation` _camera (`SplineComponent.FindLocationClosestToWorldLocation` _spline _returnvalue_2 "World") false false)
  (set `self.cameraRightVector` (`KismetMathLibrary.GetRightVector` _returnvalue))
  (set `self.cameraForwardVector` (`KismetMathLibrary.GetForwardVector` _returnvalue)))

(fn `UserConstructionScript`)