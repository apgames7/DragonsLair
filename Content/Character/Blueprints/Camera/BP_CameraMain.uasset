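; Main level camera that takes over the player's view and rides the CameraPath spline as the player moves.
; Each tick it snaps to the spline point closest to a forward offset from the player.
; It takes yaw from the spline until a trigger switches it to facing the player.
; Trigger volumes also enable collision against backtracking and reveal the boss health widget, created hidden at BeginPlay.
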(event `self.ReceiveBeginPlay`
  ; Set Camera view + Create widgets from blueprints
  (`PlayerController.SetViewTargetWithBlend` (`GameplayStatics.GetPlayerController` 0) self 0.0 "VTBlend_Linear" 0.0 false)
  (bind _returnvalue (`|CreateWidget` "/Game/UI/Widget/WBP_BossHealth.WBP_BossHealth_C"))
  (`UserWidget.AddToViewport` _returnvalue 0)
  (`Widget.SetIsEnabled` _returnvalue false)
  (`Widget.SetVisibility` _returnvalue "Hidden"))

(event `self.ReceiveTick`
  (params (DeltaSeconds :type "Float (single-precision)"))
  (bind (_returnvalue_roll _returnvalue_pitch) (`KismetMathLibrary.BreakRotator` (`SceneComponent.K2_GetComponentRotation` (`self.Camera`))))
  ; Movement + Rotation
  (`|ExecutionSequence`
    (:`then_0`
      (bind (_returnvalue_roll_2 _returnvalue_yaw) (`self.RotationToPlayer`)))
    (:`then_1`
      (bind (_returnvalue_yaw_2 _returnvalue) (`self.GetRotationLocation`)))
    (:`then_2`
      (if (`self.isRotateToPlayer`)
        (`SceneComponent.K2_SetWorldRotation` (`self.Camera`) (`KismetMathLibrary.MakeRotator` _returnvalue_roll_2 0.0 _returnvalue_yaw) false false)
        (else
          (`SceneComponent.K2_SetWorldRotation` (`self.Camera`) (`KismetMathLibrary.MakeRotator` _returnvalue_roll _returnvalue_pitch _returnvalue_yaw_2) false false)))
      (`SceneComponent.K2_SetWorldLocation` (`self.Camera`) _returnvalue false false))))

(event `self.StopPlayerFromGoingBack.OnComponentBeginOverlap`
  (params (OverlappedComponent :type "PrimitiveComponent Object Reference") (OtherActor :type "Actor Object Reference") (OtherComp :type "PrimitiveComponent Object Reference") (OtherBodyIndex :type Integer) (bFromSweep :type Boolean) (SweepResult :type "HitResult Structure (by ref)"))
  ; Triggers
  (if (`self.ActorHasTag` OtherActor "Player")
    (set `self.isRotateToPlayer` true)
    (`PrimitiveComponent.SetCollisionEnabled` (`self.StopPlayerFromGoingBack`) "QueryAndPhysics")))

(event `self.BossRoom.OnComponentBeginOverlap`
  (params (OverlappedComponent :type "PrimitiveComponent Object Reference") (OtherActor :type "Actor Object Reference") (OtherComp :type "PrimitiveComponent Object Reference") (OtherBodyIndex :type Integer) (bFromSweep :type Boolean) (SweepResult :type "HitResult Structure (by ref)"))
  ; Triggers
  (if (`self.ActorHasTag` OtherActor "Player")
    (bind _foundwidgets (`WidgetBlueprintLibrary.GetAllWidgetsOfClass` "/Game/UI/Widget/WBP_BossHealth.WBP_BossHealth_C"))
    (for _array_element _foundwidgets
      (`Widget.SetIsEnabled` _array_element true :!label _label)
      (`Widget.SetVisibility` _array_element "Visible"))
    (goto _label)))

(event `self.RotateTorwardsPlayer.OnComponentBeginOverlap`
  (params (OverlappedComponent :type "PrimitiveComponent Object Reference") (OtherActor :type "Actor Object Reference") (OtherComp :type "PrimitiveComponent Object Reference") (OtherBodyIndex :type Integer) (bFromSweep :type Boolean) (SweepResult :type "HitResult Structure (by ref)"))
  ; Triggers
  (if (`self.ActorHasTag` OtherActor "Player")
    (set `self.isRotateToPlayer` true)))

(fn `GetRotationLocation`
  (returns (ReturnValue_Yaw :type "Float (single-precision)") (ReturnValue :type "Vector Structure"))
  (bind _camerapath (`self.CameraPath`))
  (bind _returnvalue (+ (* (`KismetMathLibrary.GetForwardVector` (`SceneComponent.K2_GetComponentRotation` (`self.Camera`))) (`self.distanceToPlayer`)) (`self.K2_GetActorLocation` (`GameplayStatics.GetPlayerCharacter` 0))))
  (bind (_returnvalue_roll _returnvalue_pitch _returnvalue_yaw) (`KismetMathLibrary.BreakRotator` (`SplineComponent.FindRotationClosestToWorldLocation` _camerapath _returnvalue "World")))
  (return _returnvalue_yaw (`SplineComponent.FindLocationClosestToWorldLocation` _camerapath _returnvalue "World")))

(fn `RotationToPlayer`
  (returns (ReturnValue_Roll :type "Float (single-precision)") (ReturnValue_Yaw :type "Float (single-precision)"))
  (bind (_returnvalue_roll _returnvalue_pitch _returnvalue_yaw) (`KismetMathLibrary.BreakRotator` (`KismetMathLibrary.FindLookAtRotation` (`SceneComponent.K2_GetComponentLocation` (`self.Camera`)) (`self.K2_GetActorLocation` (`GameplayStatics.GetPlayerCharacter` 0)))))
  (return _returnvalue_roll _returnvalue_yaw))

(fn `UserConstructionScript`)