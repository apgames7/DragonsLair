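; BP_FollowSideCamera is a side-view camera actor that takes over the player's view.
; When a "Player"-tagged actor overlaps SwitchCameraTrigger, it blends the player controller's view to itself, finds BP_DragonPlayer and sets its SideViewCamera flag.
; Logic to follow the player mesh along X with a swept move exists but is disconnected; Tick is empty, so the actor does not follow.
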(event `self.ReceiveTick`
  (params (DeltaSeconds :type "Float (single-precision)")))

(event `self.SwitchCameraTrigger.OnComponentBeginOverlap`
  (params (OverlappedComponent :type "PrimitiveComponent Object Reference") (OtherActor :type "Actor Object Reference") (OtherComp :type "PrimitiveComponent Object Reference") (OtherBodyIndex :type Integer) (bFromSweep :type Boolean) (SweepResult :type "HitResult Structure (by ref)"))
  (if (`self.ActorHasTag` OtherActor "Player")
    (`PlayerController.SetViewTargetWithBlend` (`GameplayStatics.GetPlayerController` 0) self 0.0 "VTBlend_Linear" 0.0 false)
    (bind _returnvalue (`GameplayStatics.GetActorOfClass` "/Game/Character/Blueprints/Player/BP_DragonPlayer.BP_DragonPlayer_C"))
    (set `self.PlayerRef` _returnvalue)
    (bind _playerref (`self.PlayerRef`)
      (:`then`
        (set `/Game/Character/Blueprints/Player/BP_DragonPlayer.sideViewCamera` true _playerref))
      (:`else`))))

(fn `UserConstructionScript`)