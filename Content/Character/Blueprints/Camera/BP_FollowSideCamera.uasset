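; BP_FollowSideCamera is a side-view camera actor that takes over the player's view when its SwitchCameraTrigger is overlapped.
; On overlap, it blends player 0's view target to itself, finds BP_DragonPlayer and sets that player's SideViewCamera flag.
; While the flag is set, Tick moves the actor with sweep to match the player mesh's world X, keeping its own Y and Z.
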(event `self.ReceiveTick`
  (params (DeltaSeconds :type "Float (single-precision)"))
  (bind (_returnvalue_x _returnvalue_y _returnvalue_z) (`KismetMathLibrary.BreakVector` (`self.K2_GetActorLocation`)))
  (if (`/Game/Character/Blueprints/Player/BP_DragonPlayer.sideViewCamera` (stale `self.SwitchCameraTrigger.OnComponentBeginOverlap` _returnvalue))
    (bind _returnvalue_x_2 (`KismetMathLibrary.BreakVector` (`SceneComponent.K2_GetComponentLocation` (`Character.Mesh` (stale `self.SwitchCameraTrigger.OnComponentBeginOverlap` _returnvalue)))))
    (`self.K2_SetActorLocation` (`KismetMathLibrary.MakeVector` _returnvalue_x_2 _returnvalue_y _returnvalue_z) true)))

(event `self.SwitchCameraTrigger.OnComponentBeginOverlap`
  (params (OverlappedComponent :type "PrimitiveComponent Object Reference") (OtherActor :type "Actor Object Reference") (OtherComp :type "PrimitiveComponent Object Reference") (OtherBodyIndex :type Integer) (bFromSweep :type Boolean) (SweepResult :type "HitResult Structure (by ref)"))
  (`PlayerController.SetViewTargetWithBlend` (`GameplayStatics.GetPlayerController` 0) self 0.0 "VTBlend_Linear" 0.0 false)
  (bind _returnvalue (`GameplayStatics.GetActorOfClass` "/Game/Character/Blueprints/Player/BP_DragonPlayer.BP_DragonPlayer_C"))
  (set `/Game/Character/Blueprints/Player/BP_DragonPlayer.sideViewCamera` true _returnvalue))

(fn `UserConstructionScript`)