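; BP_Weapon is a weapon pickup that unlocks the sword for the player.
; On any actor overlap it prints a debug string, casts player character 0 to BP_DragonPlayer, sets CanHaveSword and destroys itself.
; The overlapping actor is never checked, so any overlapping actor grants the player the sword, provided the cast succeeds.
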(event `self.ReceiveActorBeginOverlap`
  (params (OtherActor :type "Actor Object Reference"))
  (`parent.ReceiveActorBeginOverlap` OtherActor)
  (`KismetSystemLibrary.PrintString` "Overlap")
  (bind _asbp_dragon_player (cast `/Game/Character/Blueprints/Player/BP_DragonPlayer` (`GameplayStatics.GetPlayerCharacter` 0)))
  (set `/Game/Character/Blueprints/Player/BP_DragonPlayer.canHaveSword` true _asbp_dragon_player)
  (`self.K2_DestroyActor`))

(fn `UserConstructionScript`
  (`parent.UserConstructionScript`))