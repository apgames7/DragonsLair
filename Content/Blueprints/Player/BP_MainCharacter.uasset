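; Player character Blueprint that handles a sword attack on a single enemy and the player's lose condition.
; BeginPlay caches one BP_EnemyBackup, which IA_DragonAttack damages when its HitBox overlaps AttackBox and both attack flags allow it.
; Each hit applies a horizontal impulse along the enemy-to-player direction, removes a life and starts a short cooldown.
; Tick polls Lives and loads DeathMenu as a level instance every frame they are depleted.
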(event `self.ReceiveBeginPlay`
  (bind _returnvalue (`GameplayStatics.GetActorOfClass` "/Game/Blueprints/Enemies/BP_EnemyBackup.BP_EnemyBackup_C"))
  (set `self.Enemy` _returnvalue))

(event `self.ReceiveTick`
  (params (DeltaSeconds :type "Float (single-precision)"))
  ; Lose Condition
  (if (<= (`self.lives`) 0.0)
    (`LevelStreamingDynamic.LoadLevelInstance` "DeathMenu" (0.0 0.0 0.0) (struct) "" null)
    (`KismetSystemLibrary.PrintString` "lose")))

(event `EnhancedInput|/Game/Input/InputActions/IA_DragonAttack`
  (params (ActionValue :type Boolean) (ElapsedSeconds :type "Float (double-precision)") (TriggeredSeconds :type "Float (double-precision)") (InputAction :type "InputAction Object Reference" :default "/Game/Input/InputActions/IA_DragonAttack.IA_DragonAttack"))
  (bind _enemy (`self.Enemy`))
  ; Attack Condition
  (:`Triggered`
    (if (and (and (`PrimitiveComponent.IsOverlappingComponent` (`/Game/Blueprints/Enemies/BP_EnemyBackup.hitBox` (`self.Enemy`)) (`self.attackBox`)) (`self.canAttack`)) (`self.canHaveSword`))
      ; Add Knockback
      (`CharacterMovementComponent.AddImpulse` (`Character.CharacterMovement` (`self.Enemy`)) (* (`KismetMathLibrary.Normal` (- (`SceneComponent.K2_GetComponentLocation` (`self.Mesh`)) (`SceneComponent.K2_GetComponentLocation` (`Character.Mesh` (`self.Enemy`))))) (7000.0 7000.0 0.0)) false)
      ; Attack
      (set `/Game/Blueprints/Enemies/BP_EnemyBackup.lives` (- (`/Game/Blueprints/Enemies/BP_EnemyBackup.lives` _enemy) 1.0) _enemy)
      (set `self.canAttack` false)
      (`KismetSystemLibrary.Delay` 1.0)
      (set `self.canAttack` true))))

(fn `UserConstructionScript`)