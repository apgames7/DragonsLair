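; Follow camera actor that becomes the player's view target and slides along a spline to track the player character.
; Each tick it snaps to the spline point closest to the player plus a forward offset, taking yaw from the spline or, once triggered, facing the player.
; Overlap volumes switch on player-facing rotation, enable collision behind the player, or reveal the boss health widget created hidden at BeginPlay.
; Earlier offset and rail-rig approaches remain unconnected.
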(event `self.ReceiveBeginPlay`
  (`PlayerController.SetViewTargetWithBlend` (`GameplayStatics.GetPlayerController` 0) self 0.0 "VTBlend_Linear" 0.0 false)
  (bind _returnvalue (`|CreateWidget` "/Game/UI/Widget/WBP_BossHealth.WBP_BossHealth_C"))
  (`UserWidget.AddToViewport` _returnvalue 0)
  (`Widget.SetIsEnabled` _returnvalue false)
  (`Widget.SetVisibility` _returnvalue "Hidden"))

(event `self.ReceiveTick`
  (params (DeltaSeconds :type "Float (single-precision)"))
  (bind _spline (`self.Spline`))
  (bind _camera (`self.Camera`))
  (bind _returnvalue (`SceneComponent.K2_GetComponentRotation` (`self.Camera`)))
  (bind (_returnvalue_roll _returnvalue_pitch) (`KismetMathLibrary.BreakRotator` (`SceneComponent.K2_GetComponentRotation` _camera)))
  (bind (_returnvalue_roll_2 _returnvalue_pitch_2 _returnvalue_yaw) (`KismetMathLibrary.BreakRotator` (`KismetMathLibrary.FindLookAtRotation` (`SceneComponent.K2_GetComponentLocation` _camera) (`self.K2_GetActorLocation` (`GameplayStatics.GetPlayerCharacter` 0)))))
  (bind _returnvalue_2 (+ (* (`KismetMathLibrary.GetForwardVector` (`SceneComponent.K2_GetComponentRotation` (`self.Camera`))) (`self.distanceToPlayer`)) (`self.K2_GetActorLocation` (`GameplayStatics.GetPlayerCharacter` 0))))
  (bind (_returnvalue_roll_3 _returnvalue_pitch_3 _returnvalue_yaw_2) (`KismetMathLibrary.BreakRotator` (`SplineComponent.FindRotationClosestToWorldLocation` _spline _returnvalue_2 "World")))
  ; Camera move on spline
  (if (`self.isRotateToPlayer`)
    ; Camera Rotation
    (`SceneComponent.K2_SetWorldRotation` _camera (`KismetMathLibrary.MakeRotator` _returnvalue_roll_2 0.0 _returnvalue_yaw) false false)
    (else
      (`SceneComponent.K2_SetWorldRotation` _camera (`KismetMathLibrary.MakeRotator` _returnvalue_roll _returnvalue_pitch _returnvalue_yaw_2) false false)))
  (`SceneComponent.K2_SetWorldLocation` _camera (`SplineComponent.FindLocationClosestToWorldLocation` _spline _returnvalue_2 "World") false false)
  (set `self.cameraRightVector` (`KismetMathLibrary.GetRightVector` _returnvalue))
  (set `self.cameraForwardVector` (`KismetMathLibrary.GetForwardVector` _returnvalue)))

(event `self.StopPlayerFromGoingBack.OnComponentBeginOverlap`
  (params (OverlappedComponent :type "PrimitiveComponent Object Reference") (OtherActor :type "Actor Object Reference") (OtherComp :type "PrimitiveComponent Object Reference") (OtherBodyIndex :type Integer) (bFromSweep :type Boolean) (SweepResult :type "HitResult Structure (by ref)"))
  (if (`self.ActorHasTag` OtherActor "Player")
    (set `self.isRotateToPlayer` true)
    (`PrimitiveComponent.SetCollisionEnabled` (`self.StopPlayerFromGoingBack`) "QueryAndPhysics")))

(event `self.InEnemyFight.OnComponentBeginOverlap`
  (params (OverlappedComponent :type "PrimitiveComponent Object Reference") (OtherActor :type "Actor Object Reference") (OtherComp :type "PrimitiveComponent Object Reference") (OtherBodyIndex :type Integer) (bFromSweep :type Boolean) (SweepResult :type "HitResult Structure (by ref)"))
  (if (`self.ActorHasTag` OtherActor "Player")
    (bind _foundwidgets (`WidgetBlueprintLibrary.GetAllWidgetsOfClass` "/Game/UI/Widget/WBP_BossHealth.WBP_BossHealth_C"))
    (`KismetSystemLibrary.PrintString` "triggered")
    (for _array_element _foundwidgets
      (`Widget.SetIsEnabled` _array_element true :!label _label)
      (`Widget.SetVisibility` _array_element "Visible")
      (`KismetSystemLibrary.PrintString` "testHello"))
    (goto _label)))

(event `self.CameraRotateTowardsPlayer.OnComponentBeginOverlap`
  (params (OverlappedComponent :type "PrimitiveComponent Object Reference") (OtherActor :type "Actor Object Reference") (OtherComp :type "PrimitiveComponent Object Reference") (OtherBodyIndex :type Integer) (bFromSweep :type Boolean) (SweepResult :type "HitResult Structure (by ref)"))
  (if (`self.ActorHasTag` OtherActor "Player")
    (set `self.isRotateToPlayer` true)
    (`KismetSystemLibrary.PrintString` "overlapped")))

(fn `UserConstructionScript`)