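; Enemy actor that chases and attacks the DragonCharacter player, with a win condition for bosses.
; Tick measures distance to the player's mesh and moves toward it when between attack and chase range.
; Inside attack range, an attack box overlap costs the player a life and plays a spider animation, with a delay-based cooldown.
; While chasing, a Boss-tagged enemy with one or fewer lives loads the WinMenu level instance.
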(event `self.ReceiveBeginPlay`
  (bind _returnvalue (`GameplayStatics.GetActorOfClass` "/Script/DragonsLair.DragonCharacter"))
  (set `self.Player` _returnvalue))

(event `self.ReceiveTick`
  (params (DeltaSeconds :type "Float (single-precision)"))
  (bind _returnvalue (- (`SceneComponent.K2_GetComponentLocation` (`Character.Mesh` (`self.Player`))) (`self.K2_GetActorLocation`)))
  (bind _returnvalue_2 (`KismetMathLibrary.VSize` _returnvalue))
  ; Move
  (set `self.lengthBetweenEnemyPlayer` _returnvalue_2)
  (if (and (< _returnvalue_2 (`self.chaseLength`)) (> _returnvalue_2 (`self.attackLength`)))
    (`self.AddMovementInput` (`KismetMathLibrary.Normal` _returnvalue) (`self.speed`) true)
    ; Win Condition
    (if (and (`self.ActorHasTag` "Boss") (<= (`self.lives`) 1.0))
      (`LevelStreamingDynamic.LoadLevelInstance` "WinMenu" (0.0 0.0 0.0) (struct) "" null)
      (`KismetSystemLibrary.PrintString` "win")
      (else
        ; Attack
        (if (and (and (< (`self.lengthBetweenEnemyPlayer`) (`self.attackLength`)) (`self.canAttack`)) (`PrimitiveComponent.IsOverlappingComponent` (`Character.CapsuleComponent` (`self.Player`)) (`self.attackBox`))) :!label _label
          (set `self.canAttack` false)
          (set `DragonCharacter.lives` (- (`DragonCharacter.lives` (`self.Player`)) 1.0) (`self.Player`))
          (`SkeletalMeshComponent.PlayAnimation` (`self.Mesh`) "/Game/Art/Characters/Spider/Spider_360/Wolf_Spider_attack_360Wolf_Spider_Armature_Wolf_Spider_Armature_Spider_Attacking.Wolf_Spider_attack_360Wolf_Spider_Armature_Wolf_Spider_Armature_Spider_Attacking" false)
          (`KismetSystemLibrary.Delay` 0.5)
          (`SkeletalMeshComponent.SetAnimationMode` (`self.Mesh`) "AnimationBlueprint" true)
          (`KismetSystemLibrary.Delay` 2.0)
          (set `self.canAttack` true))))
    (else
      (goto _label))))

(fn `UserConstructionScript`)