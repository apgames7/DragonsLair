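; BP_KnifeTrap is a one-shot trap that fires four physics-driven knives when any actor first overlaps it.
; BeginPlay derives the launch impulse from the Direction component's forward vector.
; ActivateTrap, called twice under the IsTriggered guard, enables physics, applies impulses, then destroys the trap after a short delay.
; Knife hits on Player-tagged actors share logic that removes a life from player zero's BP_MainCharacter.
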(event `self.ReceiveActorBeginOverlap`
  (params (OtherActor :type "Actor Object Reference"))
  (if (not (`self.bIsTriggered`))
    (`self.ActivateTrap`)
    (set `self.bIsTriggered` true)
    (`self.ActivateTrap`)))

(event `ActivateTrap`
  (bind _knife2 (`self.Knife2`))
  (bind _knife3 (`self.Knife3`))
  (bind _knife4 (`self.Knife4`))
  (bind _knife1 (`self.Knife1`))
  (`|ExecutionSequence`
    (:`then_0`
      (`PrimitiveComponent.SetSimulatePhysics` _knife1 true)
      (`PrimitiveComponent.SetSimulatePhysics` _knife2 true)
      (`PrimitiveComponent.SetSimulatePhysics` _knife3 true)
      (`PrimitiveComponent.SetSimulatePhysics` _knife4 true))
    (:`then_1`
      (`PrimitiveComponent.AddImpulse` _knife1 (`self.KnifeMagnitude`) "None" false)
      (`PrimitiveComponent.AddImpulse` _knife2 (`self.KnifeMagnitude`) "None" false)
      (`PrimitiveComponent.AddImpulse` _knife3 (`self.KnifeMagnitude`) "None" false)
      (`PrimitiveComponent.AddImpulse` _knife4 (`self.KnifeMagnitude`) "None" false)
      (`KismetSystemLibrary.Delay` 1.0)
      (`self.K2_DestroyActor`))))

(event `self.ReceiveBeginPlay`
  ; Create direction of Knifes
  (set `self.KnifeMagnitude` (* (`SceneComponent.GetForwardVector` (`self.Direction`)) 2500.0)))

(event `self.Knife4.OnComponentHit`
  (params (HitComponent :type "PrimitiveComponent Object Reference") (OtherActor :type "Actor Object Reference") (OtherComp :type "PrimitiveComponent Object Reference") (NormalImpulse :type "Vector Structure") (Hit :type "HitResult Structure (by ref)"))
  (if (`self.ActorHasTag` OtherActor "Player")
    (bind _asbp_main_character (cast `/Game/Blueprints/Player/BP_MainCharacter` (`GameplayStatics.GetPlayerCharacter` 0) :!label _label))
    (set `DragonCharacter.lives` (- (`DragonCharacter.lives` _asbp_main_character) 1.0) _asbp_main_character)))

(event `self.Knife3.OnComponentHit`
  (params (HitComponent :type "PrimitiveComponent Object Reference") (OtherActor :type "Actor Object Reference") (OtherComp :type "PrimitiveComponent Object Reference") (NormalImpulse :type "Vector Structure") (Hit :type "HitResult Structure (by ref)"))
  (if (`self.ActorHasTag` OtherActor "Player")
    (goto _label)))

(event `self.Knife2.OnComponentHit`
  (params (HitComponent :type "PrimitiveComponent Object Reference") (OtherActor :type "Actor Object Reference") (OtherComp :type "PrimitiveComponent Object Reference") (NormalImpulse :type "Vector Structure") (Hit :type "HitResult Structure (by ref)"))
  (if (`self.ActorHasTag` OtherActor "Player")
    (goto _label)))

(event `self.Knife1.OnComponentHit`
  (params (HitComponent :type "PrimitiveComponent Object Reference") (OtherActor :type "Actor Object Reference") (OtherComp :type "PrimitiveComponent Object Reference") (NormalImpulse :type "Vector Structure") (Hit :type "HitResult Structure (by ref)"))
  (if (`self.ActorHasTag` OtherActor "Player")
    (goto _label)))

(fn `UserConstructionScript`)