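; Health potion pickup that grants the player an extra life on contact.
; On overlap with an actor tagged Player, it casts player character 0, rather than the overlapping actor, to DragonCharacter.
; If the cast succeeds, it increments that character's Lives and destroys itself.
; BeginPlay and Tick are disabled, and the construction script only calls its parent.
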(event `self.ReceiveActorBeginOverlap`
  (params (OtherActor :type "Actor Object Reference"))
  (`parent.ReceiveActorBeginOverlap` OtherActor)
  (if (`self.ActorHasTag` OtherActor "Player")
    (bind _asdragon_character (cast `DragonCharacter` (`GameplayStatics.GetPlayerCharacter` 0)))
    (set `DragonCharacter.lives` (+ (`DragonCharacter.lives` _asdragon_character) 1.0) _asdragon_character)
    (`self.K2_DestroyActor`)))

(fn `UserConstructionScript`
  (`parent.UserConstructionScript`))