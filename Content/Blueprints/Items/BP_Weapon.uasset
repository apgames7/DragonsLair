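; BP_Weapon is a pickup item that grants the player the ability to have a sword.
; On actor overlap, it checks for the Player tag and casts the other actor to DragonCharacter.
; It then sets that character's CanHaveSword flag and destroys itself.
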(event `self.ReceiveActorBeginOverlap`
  (params (OtherActor :type "Actor Object Reference"))
  (if (`self.ActorHasTag` OtherActor "Player")
    (bind _asdragon_character (cast `DragonCharacter` OtherActor))
    (set `DragonCharacter.canHaveSword` true _asdragon_character)
    (`self.K2_DestroyActor`)))

(fn `UserConstructionScript`
  (`parent.UserConstructionScript`))